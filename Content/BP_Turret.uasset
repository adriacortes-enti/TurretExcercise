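; BP_Turret is a turret actor whose top turns to track the third-person character.
; BeginPlay caches the first BP_ThirdPersonCharacter found in the level as the target.
; Each Tick derives yaw and pitch to the target with Atan2, keeping roll at zero.
; It eases toward them with a fixed-alpha float Lerp, so smoothing is frame-rate dependent and does not handle angle wraparound.
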(event `self.ReceiveBeginPlay`
  (bind _returnvalue (`GameplayStatics.GetActorOfClass` "/Game/ThirdPerson/Blueprints/BP_ThirdPersonCharacter.BP_ThirdPersonCharacter_C"))
  (set `self.TargetBlueprint` _returnvalue))

(event `self.ReceiveTick`
  (params (DeltaSeconds :type "Float (single-precision)"))
  (bind (_returnvalue_roll _returnvalue_pitch _returnvalue_yaw) (`KismetMathLibrary.BreakRotator` (`SceneComponent.K2_GetComponentRotation` (`self.TurretTop`))))
  (bind (_returnvalue_x _returnvalue_y _returnvalue_z) (`KismetMathLibrary.BreakVector` (- (`self.K2_GetActorLocation` (`self.TargetBlueprint`)) (`SceneComponent.K2_GetComponentLocation` (`self.TurretTop`)))))
  (`SceneComponent.K2_SetWorldRotation` (`self.TurretTop`) (`KismetMathLibrary.MakeRotator` 0.0 (`KismetMathLibrary.Lerp` _returnvalue_pitch (`KismetMathLibrary.DegAtan2` _returnvalue_z (`KismetMathLibrary.VSize` (`KismetMathLibrary.MakeVector` _returnvalue_x _returnvalue_y))) 0.05) (`KismetMathLibrary.Lerp` _returnvalue_yaw (`KismetMathLibrary.DegAtan2` _returnvalue_y _returnvalue_x) 0.05)) false false))

(fn `UserConstructionScript`)